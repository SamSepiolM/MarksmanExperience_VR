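; Serial bridge Blueprint between the indoor shooting range and an Arduino gyroscope controller with a fire button.
; StartArduino and CloseArduino manage the COM port with start/stop commands, and WriteArduino sends arbitrary lines.
; GetArduinoData, gated on the Calibrado flag, parses comma-separated serial readings into a rotator and trigger state.
; Event graph logic for connection, timed calibration, actor rotation and closing is disconnected, so nothing here sets Calibrado at runtime.
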(event EventBeginPlay)

(event Collision|EventActorBeginOverlap
  (params (OtherActor :type Actor%20Object%20Reference)))

(event EventTick
  (params (DeltaSeconds :type Float%20%28single-precision%29)))

(event EventEndPlay
  (params (EndPlayReason :type EEndPlayReason%20Enum :default "Destroyed")))

(fn ConstructionScript)

(fn StartArduino
  (params (Port :type Integer) (BaudRate :type Integer))
  (bind (_bopened _returnvalue) (Class|Serial|OpenComPort Port BaudRate))
  (bind _output_get (Variables|Default|SetArduinoOpened _bopened))
  (if _output_get
    (Development|PrintString "Ya conecte con Arduino")
    (bind _output_get_2 (Variables|Default|SetArduinoData _returnvalue))
    (Class|Serial|Println _output_get_2 "1")
    (else
      (Development|PrintString "No se puede conectar con Arduino")))
  (return (Variables|Default|GetArduinoOpened)))

(fn GetArduinoData
  (bind _arduinodata (Variables|Default|GetArduinoData)
    (:then
      (if (and (Class|Serial|IsOpened _arduinodata) (Variables|Default|GetCalibrado))
        (bind (_bsuccess _returnvalue) (Class|Serial|ReadString _arduinodata))
        (if _bsuccess
          (Variables|Default|SetData? true)
          (else
            (Variables|Default|SetData? false)))
        (return (Math|Rotator|MakeRotator (Math|Conversions|ToFloat(Integer) (Utilities|Array|Get(acopy) (Utilities|String|ParseIntoArray _returnvalue "," false) 1)) (Math|Conversions|ToFloat(Integer) (Utilities|Array|Get(acopy) (Utilities|String|ParseIntoArray _returnvalue "," false))) (Math|Conversions|ToFloat(Integer) (Utilities|Array|Get(acopy) (Utilities|String|ParseIntoArray _returnvalue "," false) 2))) (Variables|Default|GetData?) (== (Math|Conversions|ToFloat(Integer) (Utilities|Array|Get(acopy) (Utilities|String|ParseIntoArray _returnvalue "," false) 3)) 1.0))))
    (:else)))

(fn CloseArduino
  (bind _arduinodata (Variables|Default|GetArduinoData))
  (if (Variables|Default|GetArduinoOpened)
    (Class|Serial|Println _arduinodata "0")
    (Class|Serial|Close _arduinodata)))

(fn WriteArduino
  (params (String :type String))
  (if (Variables|Default|GetArduinoOpened)
    (Class|Serial|Println (Variables|Default|GetArduinoData) String)))